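; BP_Key is an interactable key pickup that records which key the player has acquired.
; On BeginPlay it casts the game mode to GameMode_lb and caches it.
; Interact writes its KeyNumber into the game mode's Keys, then prints an acquisition message using the matching entry in Names.
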(event `self.ReceiveBeginPlay`
  (bind _asgame_mode_lb (cast `/Game/ThirdPerson/Maps/Midterm/GameMode_lb` (`GameplayStatics.GetGameMode`)))
  (set `self.As Game Mode Lb` _asgame_mode_lb))

(event `self.Interact`
  (bind _output_get (set `/Game/ThirdPerson/Maps/Midterm/GameMode_lb.Keys` (`self.Key Number`) (`self.As Game Mode Lb`)))
  (`KismetSystemLibrary.PrintString` (`KismetStringLibrary.Concat_StrStr` "Key" (`|GetArrayItem` (`self.Names`) _output_get) "Acquired")))

(fn `UserConstructionScript`)